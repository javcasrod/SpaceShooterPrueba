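; BP_SpaceS_Ammo is a projectile actor that flies straight along its forward vector and reacts when it hits a Pawn.
; Tick moves it by Speed scaled by delta time, without sweep, so hit detection relies on actor overlap.
; Overlapping a Pawn spawns an emitter at its location, plays the Laser_Pull sound and destroys the actor after a short delay.
; It applies no damage itself.
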(event `self.ReceiveActorBeginOverlap`
  (params (OtherActor :type "Actor Object Reference"))
  (cast `Pawn` OtherActor)
  (`GameplayStatics.SpawnEmitterAtLocation` null (`self.K2_GetActorLocation`))
  (`GameplayStatics.PlaySound2D` "/Engine/VREditor/Sounds/UI/Laser_Pull.Laser_Pull" 1.0 1.0 0.0 null null)
  (`KismetSystemLibrary.Delay` 0.5)
  (`self.K2_DestroyActor`))

(event `self.ReceiveTick`
  (params (DeltaSeconds :type "Float (single-precision)"))
  (`self.K2_SetActorLocation` (+ (`self.K2_GetActorLocation`) (* (`self.GetActorForwardVector`) (* DeltaSeconds (`self.Speed`))))))

(fn `UserConstructionScript`)